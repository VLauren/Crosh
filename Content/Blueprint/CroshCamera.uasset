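; CroshCamera is a follow-camera actor that tracks the CroshBP player along X and Z.
; On BeginPlay it takes the first CroshBP in the level and stores its starting X and Z distance from it as an offset.
; Each Tick it moves to the player's position plus that offset, setting only X and Z, so sideways Y movement is not followed.
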(event `self.ReceiveBeginPlay`
  (bind _outactors (`GameplayStatics.GetAllActorsOfClass` "/Game/Blueprint/CroshBP.CroshBP_C"))
  (bind _output_get (set `self.Player` (`|GetArrayItem` _outactors)))
  (bind (_returnvalue_x _returnvalue_y _returnvalue_z) (`KismetMathLibrary.BreakVector` (- (`self.K2_GetActorLocation`) (`self.K2_GetActorLocation` _output_get))))
  (set `self.Offset` (`KismetMathLibrary.MakeVector` _returnvalue_x 0.0 _returnvalue_z)))

(event `self.ReceiveTick`
  (params (DeltaSeconds :type "Float (single-precision)"))
  (bind (_returnvalue_x _returnvalue_y _returnvalue_z) (`KismetMathLibrary.BreakVector` (+ (`self.K2_GetActorLocation` (`self.Player`)) (`self.Offset`))))
  (`self.K2_SetActorLocation` (`KismetMathLibrary.MakeVector` _returnvalue_x 0.0 _returnvalue_z)))

(fn `UserConstructionScript`)